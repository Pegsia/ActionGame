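; Explosive_BP is a networked explosive actor that detonates automatically a few seconds after it spawns.
; On BeginPlay, only the authority starts the fuse timer, which calls Explode to trigger MulticastExplode and set a short lifespan for cleanup.
; MulticastExplode fires the RadialForce impulse, prints a debug message, hides the actor and disables its collision.
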(event `self.ReceiveBeginPlay`
  (`/Engine/EditorBlueprintResources/ActorMacros.Switch Has Authority`
    (:`Authority`
      (`KismetSystemLibrary.K2_SetTimerDelegate` (delegate `Explode`) 4.0))))

(event `Explode`
  (`self.MulticastExplode`)
  (`self.SetLifeSpan` 2.0))

(event `MulticastExplode`
  (`KismetSystemLibrary.PrintString` "Explode" true true (struct :`R` 1.0 :`B` 0.037474 :`A` 1.0) 5.0)
  (`RadialForceComponent.FireImpulse` (`self.RadialForce`))
  (`self.SetActorHiddenInGame` true)
  (`self.SetActorEnableCollision` false))

(fn `UserConstructionScript`)
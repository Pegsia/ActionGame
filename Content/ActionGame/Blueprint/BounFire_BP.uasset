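; Bonfire save point that lights when interacted with and saves the world.
; Interact sets the FireActive flag, calls WriteSaveGame on the ioGameModeBase game mode and prints a confirmation.
; The flag's RepNotify and OnActorLoaded both run UpdateParticleSys, which calls Activate on the fire particle system with the flag as its argument.
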(event `UpdateParticleSys`
  (`ActorComponent.Activate` (`self.ParticleSystem`) (`self.bFireActive`)))

(event `TioGameplayInterface.Interact`
  (params (InsgitatorPawn :type "Pawn Object Reference"))
  (set `self.bFireActive` true)
  (`TioGameModeBase.WriteSaveGame` (cast `TioGameModeBase` (`GameplayStatics.GetGameMode`) :!pure true))
  (`KismetSystemLibrary.PrintString` "World Saved"))

(event `TioGameplayInterface.OnActorLoaded`
  (`self.UpdateParticleSys`))

(fn `OnRep_bFireActive`
  (`self.UpdateParticleSys`))

(fn `UserConstructionScript`)